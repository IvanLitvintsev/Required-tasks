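; BP_Block_Parent is a breakable block, named as a parent class, that takes damage when struck by BP_Ball.
; Each ball hit calls HitBall, which decrements Lives and either swaps the Cube material to show damage or, at zero, destroys the hit component rather than the actor.
; The construction script sets the starting Lives, so every block begins as a two-hit block.
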(event `self.ReceiveHit`
  (params (MyComp :type "PrimitiveComponent Object Reference") (Other :type "Actor Object Reference") (OtherComp :type "PrimitiveComponent Object Reference") (bSelfMoved :type Boolean) (HitLocation :type "Vector Structure") (HitNormal :type "Vector Structure") (NormalImpulse :type "Vector Structure") (Hit :type "HitResult Structure (by ref)"))
  (cast `/Game/MyGame/Blueprints/BP_Ball` Other)
  (`self.HitBall`))

(event `HitBall`
  ;[1 1 1] Уничтожение кубов и смена материала при ударе
  (bind _result (`/Engine/EditorBlueprintResources/StandardMacros.DecrementInt` (`self.Lives`))
    (:`  `
      (if (<= _result 0)
        (`ActorComponent.K2_DestroyComponent` (stale `self.ReceiveHit` MyComp))
        (else
          (`PrimitiveComponent.SetMaterial` (`self.Cube`) 0 "/Engine/EditorMaterials/Cloth/CameraLitDoubleSided.CameraLitDoubleSided"))))))

(fn `UserConstructionScript`
  (set `self.Lives` 2))
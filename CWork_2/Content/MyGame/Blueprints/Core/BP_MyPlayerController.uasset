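; Player controller that steers the player's platform pawn left and right.
; On possess it casts the pawn to BP_MyPawn and caches it, and on BeginPlay it switches to game-only input.
; The Left_Right axis offsets that pawn along world Y, scaled by Speed and delta time, with sweep enabled so collisions block movement.
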(event `self.ReceiveBeginPlay`
  ;[1 1 1] Автоматическая фикцсация на сцене при нажатии на Плей в редакторе
  (`WidgetBlueprintLibrary.SetInputMode_GameOnly` self))

(event `InputAxis|Left_Right`
  (params (AxisValue :type "Float (single-precision)"))
  ;[1 1 1] Управление платформой
  (`self.K2_AddActorWorldOffset` (`self.MyPawn`) (`KismetMathLibrary.MakeVector` 0.0 (* AxisValue (`GameplayStatics.GetWorldDeltaSeconds`) (`self.Speed`))) true false))

(event `self.ReceivePossess`
  (params (PossessedPawn :type "Pawn Object Reference"))
  (bind _asbp_my_pawn (cast `/Game/MyGame/Blueprints/Core/BP_MyPawn` PossessedPawn))
  (set `self.MyPawn` _asbp_my_pawn))

(fn `UserConstructionScript`)
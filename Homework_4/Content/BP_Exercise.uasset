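; BP_Exercise is a practice actor, a moving cube that explodes on contact.
; Tick moves it along its forward vector at a constant speed, scaled by delta time and without sweep.
; Any actor overlap spawns explosion and fire effect actors at its transform, then destroys it, with no check that the other actor is the player.
; The construction script applies the Material variable to the static mesh, and debug prints mark the main events.
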(event `self.ReceiveBeginPlay`
  (`KismetSystemLibrary.PrintString` "Hello"))

(event `self.ReceiveTick`
  (params (DeltaSeconds :type "Float (single-precision)"))
  ;[1 1 1] Actor Cube Movement
  (`self.K2_AddActorWorldOffset` (* (* (`self.GetActorForwardVector`) 50.0) DeltaSeconds)))

(event `self.ReceiveActorBeginOverlap`
  (params (OtherActor :type "Actor Object Reference"))
  ;[1 1 1] Collision with Player: Explosion & Fire
  (`|SpawnActorFromClass` "/Game/StarterContent/Blueprints/Blueprint_Effect_Explosion.Blueprint_Effect_Explosion_C" (`self.GetTransform`) "Undefined" "OverrideRootScale" null null)
  (`KismetSystemLibrary.PrintString` "Boom!")
  (`|SpawnActorFromClass` "/Game/StarterContent/Blueprints/Blueprint_Effect_Fire.Blueprint_Effect_Fire_C" (`self.GetTransform`) "Undefined" "OverrideRootScale" null null)
  (`self.K2_DestroyActor`))

(fn `UserConstructionScript`
  (locals (NewLocalVar :type "StaticMesh Object Reference" :default "/Script/Engine.StaticMesh'/Game/LevelPrototyping/Meshes/SM_Cube.SM_Cube'"))
  (`PrimitiveComponent.SetMaterial` (`self.StaticMesh`) 0 (`self.Material`))
  (`KismetSystemLibrary.PrintString` "Cunstruction Script: material changed"))